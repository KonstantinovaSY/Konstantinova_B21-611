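; BP_Buff is an Arcanoid power-up that moves a fixed step along local X each tick and is destroyed on overlapping BP_DeadZone.
; On BP_Platform overlap, random picks from Buffs are tested for SpawnNewBall, then, via a second roll, ChangeSize, so neither may apply.
; SpawnNewBall duplicates every BP_Ball and destroys the buff.
; ChangeSize widens all platforms, hides the buff, then after a delay restores the last looped platform and destroys itself.
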(event Collision|EventActorBeginOverlap
  (params (OtherActor :type Actor%20Object%20Reference))
  (bind _returnvalue (Math|Random|RandomIntegerinRange 0 1))
  (bind _initial_scale (Variables|Default|GetInitial_Scale))
  (Utilities|Casting|CastToBP_Platform OtherActor
    (:then
      (if (Utilities|Enum|Equal(Enum) (Utilities|Array|Get(acopy) (Variables|Default|GetBuffs) _returnvalue) "SpawnNewBall")
        (bind _outactors (Actor|GetAllActorsOfClass "/Game/MyLogic/Arcanoid/NewFolder/BP_Ball.BP_Ball_C"))
        (for _array_element _outactors
          (Game|SpawnActorfromClass "/Game/MyLogic/Arcanoid/NewFolder/BP_Ball.BP_Ball_C" (Transformation|GetWorldTransform (Variables|/Game/MyLogic/Arcanoid/NewFolder/BP_Ball.BP_Ball_C|GetSphere _array_element)) "Undefined" 0 0))
        (Actor|DestroyActor)
        (elif (Utilities|Enum|Equal(Enum) (Utilities|Array|Get(acopy) (Variables|Default|GetBuffs) _returnvalue) "ChangeSize")
          (bind _outactors_2 (Actor|GetAllActorsOfClass "/Game/MyLogic/Arcanoid/NewFolder/BP_Platform.BP_Platform_C"))
          (for _array_element_2 _outactors_2
            (Transformation|SetActorScale3D _array_element_2 (Math|Vector|MakeVector (* 1.5 (.x _initial_scale)) (.y _initial_scale) (.z _initial_scale))))
          (Rendering|SetActorHiddenInGame true)
          (Utilities|FlowControl|Delay 5.0)
          (Transformation|SetActorScale3D _array_element_2 (Math|Vector|MakeVector (.x _initial_scale) (.y _initial_scale) (.z _initial_scale)))
          (Actor|DestroyActor))))
    (:CastFailed
      (Utilities|Casting|CastToBP_DeadZone OtherActor)
      (Actor|DestroyActor))))

(event EventTick
  (params (DeltaSeconds :type Float%20%28single-precision%29))
  (Transformation|AddActorLocalOffset (Math|Vector|MakeVector 5.0 0.0 0.0) false false))

(fn ConstructionScript)