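; BP_Ball is the Arcanoid ball actor, moved every tick along Direction by Speed with a swept offset.
; Hitting BP_DeadZone destroys it, and the last remaining ball also pauses the game and shows BP_Menu.
; Otherwise it reflects Direction about the sweep normal, unconditionally, and resets the sphere's relative height.
; That branch adds to and prints Score when the ball's own display name equals "BP_Generator".
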(event EventTick
  (params (DeltaSeconds :type Float%20%28single-precision%29))
  (bind _sphere (Variables|Default|GetSphere))
  (bind _relativelocation (Variables|/Script/Engine.SceneComponent|GetRelativeLocation _sphere))
  (bind _sweephitresult (Transformation|AddActorWorldOffset (* (* (Variables|Default|Getdirection) (Variables|Default|Getspeed)) DeltaSeconds) true))
  (Utilities|Casting|CastToBP_DeadZone (.HitActor (Collision|BreakHitResult _sweephitresult))
    (:then
      (bind _outactors (Actor|GetAllActorsOfClass "BP_Ball_C"))
      (if (== (Utilities|Array|Length _outactors) 1)
        (Game|SetGamePaused true)
        (bind _returnvalue (UserInterface|CreateWidget "/Game/MyLogic/Arcanoid/NewFolder/BP_Menu.BP_Menu_C"))
        (UserInterface|Viewport|AddtoViewport _returnvalue 0))
      (Actor|DestroyActor))
    (:CastFailed
      (if true
        (Variables|Default|Setdirection (Math|Vector|MakeVector (.x (Math|Vector|GetReflectionVector (Variables|Default|Getdirection) (.Normal (Collision|BreakHitResult _sweephitresult)))) (.y (Math|Vector|GetReflectionVector (Variables|Default|Getdirection) (.Normal (Collision|BreakHitResult _sweephitresult)))) (.z (Math|Vector|GetReflectionVector (Variables|Default|Getdirection) (.Normal (Collision|BreakHitResult _sweephitresult))))))
        (Transformation|SetRelativeLocation _sphere (Math|Vector|MakeVector (.x _relativelocation) (.y _relativelocation) 6e+01) false false)
        (if (Utilities|Enum|Equal(Enum) (Utilities|GetDisplayName 0) "BP_Generator")
          (bind _output_get (Variables|Default|SetScore (+ (Variables|Default|GetScore) 10)))
          (Development|PrintString (Utilities|String|Append "Scroe:" (Utilities|String|ToString(Integer) _output_get)) true true "(R=1.000000,G=0.012585,B=0.000000,A=1.000000)" 5.0))))))

(fn ConstructionScript)